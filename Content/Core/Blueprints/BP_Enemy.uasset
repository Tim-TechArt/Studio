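; Enemy Blueprint that disintegrates and destroys itself when hit.
; Hit fires once: after a given delay it activates the disintegration VFX and plays a timeline that drives erosion, centered on the world-space hit point, in both the effect and two dynamic body materials.
; The construction script creates those materials uneroded; the actor is destroyed shortly after the timeline ends.
; AI chase toward the player is unconnected, and the impact-position getter returns zero.
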(event EventBeginPlay)

(event EventHit
  (params (HitPosition :type Vector :default "0, 0, 0") (Direction :type Vector :default "0, 0, 0") (Delay :type Float%20%28double-precision%29))
  (Utilities|FlowControl|DoOnce false
    (:Completed
      (Variables|Default|SetHit%20Position HitPosition)
      (Variables|Default|SetDirection Direction)
      (Utilities|FlowControl|Delay Delay)
      (Utilities|FlowControl|Sequence
        (:then_0
          (Components|Activation|Activate (Variables|Default|GetDisintegrateVFX) false))
        (:then_1
          (bind _disolve (Timeline|DisintegrateTimline Play)
            (:Update
              (Variables|Default|SetDisolve _disolve)
              (Utilities|FlowControl|Sequence
                (:then_0
                  (Niagara|SetNiagaraVariable(Vector3) (Variables|Default|GetDisintegrateVFX) "Direction" (Variables|Default|GetDirection))
                  (Effects|Components|ParticleSystem|SetFloatParameter (Variables|Default|GetDisintegrateVFX) "Erosion" (* (Variables|Default|GetDisolve) 0.1))
                  (Niagara|SetNiagaraVariable(Vector3) (Variables|Default|GetDisintegrateVFX) "HitPositionWS" (Variables|Default|GetHit%20Position)))
                (:then_1
                  (Rendering|Material|SetScalarParameterValue (Variables|Default|GetMaterial) "Erosion" (* (Variables|Default|GetDisolve) 1.8e+02) :!class /Script/Engine.MaterialInstanceDynamic)
                  (Rendering|Material|SetVectorParameterValue (Variables|Default|GetMaterial) "HitPointWS" (Math|Conversions|ToLinearColor(Vector) (Variables|Default|GetHit%20Position)) :!class /Script/Engine.MaterialInstanceDynamic)
                  (Rendering|Material|SetScalarParameterValue (Variables|Default|GetMaterial1) "Erosion" (* (Variables|Default|GetDisolve) 1.8e+02) :!class /Script/Engine.MaterialInstanceDynamic)
                  (Rendering|Material|SetVectorParameterValue (Variables|Default|GetMaterial1) "HitPointWS" (Math|Conversions|ToLinearColor(Vector) (Variables|Default|GetHit%20Position)) :!class /Script/Engine.MaterialInstanceDynamic))))
            (:Finished
              (Utilities|FlowControl|Delay 3.0)
              (Actor|DestroyActor))))))))

(fn ConstructionScript
  (Utilities|FlowControl|Sequence
    (:then_0
      (bind _returnvalue (Rendering|Material|CreateDynamicMaterialInstance (Variables|Character|GetMesh) 0 "/Game/Characters/Romero/Materials/Romero_body.Romero_body" "None" :!class /Script/Engine.PrimitiveComponent))
      (bind _output_get (Variables|Default|SetMaterial _returnvalue))
      (Rendering|Material|SetScalarParameterValue _output_get "Erosion" 0.0 :!class /Script/Engine.MaterialInstanceDynamic))
    (:then_1
      (bind _returnvalue_2 (Rendering|Material|CreateDynamicMaterialInstance (Variables|Character|GetMesh) 1 "/Game/Characters/Romero/Materials/Romero_body1.Romero_body1" "None" :!class /Script/Engine.PrimitiveComponent))
      (bind _output_get_2 (Variables|Default|SetMaterial1 _returnvalue_2))
      (Rendering|Material|SetScalarParameterValue _output_get_2 "Erosion" 0.0 :!class /Script/Engine.MaterialInstanceDynamic))))

(fn GetImpactVFXPosition
  (return "0, 0, 0"))