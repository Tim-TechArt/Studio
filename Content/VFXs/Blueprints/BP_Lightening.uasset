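; Lightning VFX actor that periodically fires random arcs from itself onto nearby surfaces.
; On Tick, after a cooldown, it line-traces along a random cone direction between min and max radius and spawns a Niagara arc to any hit.
; Optional branching traces onward from the first or previous hit, chosen by random bias and depth limit, spawning smaller arcs with depth-based spawn delays.
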(event EventBeginPlay)

(event Collision|EventActorBeginOverlap
  (params (OtherActor :type Actor%20Object%20Reference)))

(event EventTick
  (params (DeltaSeconds :type Float%20%28single-precision%29))
  (CallFunction|UpdateTraces))

(fn ConstructionScript)

(fn UpdateTraces
  (if (>= (- (Utilities|Time|GetTimeSeconds) (Variables|Default|GetLast%20Trace)) (Variables|Default|GetTrace%20Cooldown))
    ;[0.5208 0.5207 1] Calculate Start and Stop Points
    (LocalVariables|SetRandomDirection (Math|Random|RandomUnitVectorinConeinDegrees (Variables|Default|GetDirectional%20Unit%20Vector) (Variables|Default|GetDirection%20Cone%20Half%20Angle%20in%20Degrees)))
    (LocalVariables|SetTraceStartPoint (+ (Transformation|GetActorLocation) (* (LocalVariables|GetRandomDirection) (Variables|Default|GetMin%20Radius))))
    (LocalVariables|SetTraceStopPoint (+ (Transformation|GetActorLocation) (* (LocalVariables|GetRandomDirection) (Variables|Default|GetMax%20Radius))))
    ;[1 0.5011 0.4313] Trace inside radius from actor
    (bind _outhit (Collision|LineTraceByChannel (LocalVariables|GetTraceStartPoint) (LocalVariables|GetTraceStopPoint) "TraceTypeQuery1" false 0 "None"))
    (Variables|Default|SetLast%20Trace (Utilities|Time|GetTimeSeconds))
    (if (.bBlockingHit (Collision|BreakHitResult _outhit))
      (Utilities|FlowControl|Sequence
        (:then_0
          ;[0 0.5144 1] Spawn Lightning emitter and feed parameters
          (bind _returnvalue (Niagara|SpawnSystemAttached "/Game/VFXs/Particles/NS_LightningArc.NS_LightningArc" (Variables|Default|GetDefaultSceneRoot) "None" "0, 0, 0" "0, 0, 0" "KeepRelativeOffset" true))
          (Niagara|SetNiagaraVariable(Vector3) _returnvalue "BeamStartPoint" (LocalVariables|GetTraceStartPoint))
          (Niagara|SetNiagaraVariable(Vector3) _returnvalue "BeamStopPoint" (+ (.ImpactPoint (Collision|BreakHitResult _outhit)) (* (.ImpactNormal (Collision|BreakHitResult _outhit)) (LocalVariables|GetImpactOffset))))
          (Niagara|SetNiagaraVariable(Vector3) _returnvalue "ImpactNormal" (.ImpactNormal (Collision|BreakHitResult _outhit)))
          (Niagara|SetNiagaraVariable(Float) _returnvalue "Lenght" (* (.Distance (Collision|BreakHitResult _outhit)) 0.025))
          (LocalVariables|SetLast%20Hit%20With%20Offset (+ (.ImpactPoint (Collision|BreakHitResult _outhit)) (* (.ImpactNormal (Collision|BreakHitResult _outhit)) (LocalVariables|GetImpactOffset))))
          (LocalVariables|SetFirst%20Hit%20Location (.ImpactPoint (Collision|BreakHitResult _outhit)))
          (LocalVariables|SetFirst%20Hit%20Normal (.ImpactNormal (Collision|BreakHitResult _outhit))))
        (:then_1
          ;[0.7741 1 0.7502] Pre condition our loop
          (if (Variables|Default|GetBranches)
            (LocalVariables|SetRandomChoice 1.0)
            (LocalVariables|SetCurr%20Depth 0)
            (Utilities|FlowControl|ForLoopwithBreak 1 (Variables|Default|GetMax%20Branches)
              (:LoopBody
                (Utilities|FlowControl|Sequence
                  (:then_0
                    ;[0.6843 1 0.7025] Ceeping track of how deep we a branching
                    (if (or (>= (LocalVariables|GetRandomChoice) (Variables|Default|GetBranch%20Origi%20Bias)) (> (LocalVariables|GetCurr%20Depth) (Variables|Default|GetMax%20Depth)))
                      (LocalVariables|SetCurr%20Hit%20Location (LocalVariables|GetFirst%20Hit%20Location))
                      (LocalVariables|SetCurr%20Hit%20Normal (LocalVariables|GetFirst%20Hit%20Normal))
                      (LocalVariables|SetCurr%20Depth 0)
                      (else
                        (LocalVariables|SetCurr%20Hit%20Location (LocalVariables|GetLast%20Hit%20Location))
                        (LocalVariables|SetCurr%20Hit%20Normal (LocalVariables|GetLast%20Hit%20Normal))
                        (LocalVariables|SetCurr%20Depth (+ (LocalVariables|GetCurr%20Depth) 1)))))
                  (:then_1
                    (LocalVariables|SetTraceStartPoint (+ (LocalVariables|GetCurr%20Hit%20Location) (LocalVariables|GetCurr%20Hit%20Normal)))
                    (bind _outhit_2 (Collision|LineTraceByChannel (+ (LocalVariables|GetCurr%20Hit%20Location) (* (LocalVariables|GetCurr%20Hit%20Normal) (Variables|Default|GetBranch%20Offset))) (+ (+ (LocalVariables|GetCurr%20Hit%20Location) (* (LocalVariables|GetCurr%20Hit%20Normal) (Variables|Default|GetBranch%20Offset))) (* (Math|Random|RandomUnitVectorinConeinDegrees (LocalVariables|GetRandomDirection) (Variables|Default|GetBranch%20Cone%20Half%20Angle%20in%20Degrees)) (* (Variables|Default|GetMax%20Radius) 0.618))) "TraceTypeQuery1" false 0 "None"))
                    ;[0 0.5144 1] Spawb Lightning emitter and feed parameters
                    (if (.bBlockingHit (Collision|BreakHitResult _outhit_2))
                      (bind _returnvalue_2 (Niagara|SpawnSystemAttached "/Game/VFXs/Particles/NS_LightningArcPetite.NS_LightningArcPetite" (Variables|Default|GetDefaultSceneRoot) "None" "0, 0, 0" "0, 0, 0" "KeepRelativeOffset" true))
                      (Niagara|SetNiagaraVariable(Vector3) _returnvalue_2 "BeamStartPoint" (LocalVariables|GetTraceStartPoint))
                      (Niagara|SetNiagaraVariable(Float) _returnvalue_2 "SpawnDelay" (* 0.15 (+ (LocalVariables|GetCurr%20Depth) 1)))
                      (Niagara|SetNiagaraVariable(Vector3) _returnvalue_2 "BeamStopPoint" (+ (.ImpactPoint (Collision|BreakHitResult _outhit_2)) (* (.ImpactNormal (Collision|BreakHitResult _outhit_2)) (LocalVariables|GetImpactOffset))))
                      (Niagara|SetNiagaraVariable(Vector3) _returnvalue_2 "ImpactNormal" (.ImpactNormal (Collision|BreakHitResult _outhit_2)))
                      (Niagara|SetNiagaraVariable(Float) _returnvalue_2 "Lenght" (* (.Distance (Collision|BreakHitResult _outhit_2)) 0.025))
                      (LocalVariables|SetLast%20Hit%20With%20Offset (+ (.ImpactPoint (Collision|BreakHitResult _outhit_2)) (* (.ImpactNormal (Collision|BreakHitResult _outhit_2)) (LocalVariables|GetImpactOffset))))
                      (LocalVariables|SetLast%20Hit%20Location (.Location (Collision|BreakHitResult _outhit_2)))
                      (LocalVariables|SetLast%20Hit%20Normal (.ImpactNormal (Collision|BreakHitResult _outhit_2)))
                      (LocalVariables|SetRandomChoice (Math|Random|RandomFloatinRange 0.0 1.0)))))))))))))