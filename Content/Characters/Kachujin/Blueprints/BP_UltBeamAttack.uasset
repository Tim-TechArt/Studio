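; BP_UltBeamAttack is Kachujin's ultimate beam attack; FireBeam stores the mesh and material, then plays the AM_BeemMid montage.
; Its Charge Up, Beam, End and Electrify phase logic is unwired, holding time dilation, post-process and glow timelines, lightning Niagara, dissolve and camera shake.
; TraceAndHit, called from that unwired Beam phase, sphere-traces forward and sends HitMessage with delays scaled by distance from the first impact, staggering reactions.
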(event Custom|FireBeam
  (params (Mesh :type Skeletal%20Mesh%20Component%20Object%20Reference) (Material :type Material%20Instance%20Dynamic%20Object%20Reference))
  (bind _output_get (Variables|Default|SetMesh Mesh))
  (Variables|Default|SetMaterial Material)
  (Animation|Montage|PlayMontage _output_get "/Game/Characters/Kachujin/AnimationMontage/AM_BeemMid.AM_BeemMid" 1.0 0.0 ""
    (:then
      (Development|PrintString "Hello"))))

(fn ConstructionScript)

(fn TraceandHit
  (bind _mesh (Variables|Default|GetMesh))
  (bind _returnvalue (Transformation|GetWorldLocation _mesh))
  (bind _returnvalue_2 (+ _returnvalue "0.000000,0.000000,140.000000"))
  (LocalVariables|SetForward (Math|Rotator|GetRotationXVector (Transformation|GetWorldRotation (Variables|Default|GetForwardArrow))))
  (bind _outhits (Collision|MultiSphereTraceByChannel _returnvalue_2 (+ _returnvalue_2 (* (LocalVariables|GetForward) 1e+03)) 2e+01 "TraceTypeQuery3" false 0 "ForDuration"))
  (for _array_element _outhits
    (LocalVariables|SetImpact%20Point (.ImpactPoint (Collision|BreakHitResult _array_element)))
    (Utilities|FlowControl|Sequence
      (:then_0
        (Utilities|FlowControl|DoOnce false
          (:Completed
            (LocalVariables|SetLast%20Impact%20Point (LocalVariables|GetImpact%20Point)))))
      (:then_1
        (LocalVariables|SetHit%20Actor (.HitActor (Collision|BreakHitResult _array_element)))
        (Class|BPIAttackInteraction|Hit(Message) (LocalVariables|GetHit%20Actor) (LocalVariables|GetImpact%20Point) (LocalVariables|GetForward) (* (Math|Vector|Distance(Vector) (LocalVariables|GetImpact%20Point) (LocalVariables|GetLast%20Impact%20Point)) 0.0009))))))